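; Projectile actor in the Leviathan Axe weapon folder that stops and plays a hit effect after repeated overlaps.
; Its sphere counts overlaps with actors that do not implement BPI_ProjectilHit, ignoring those that do.
; From the third counted overlap onward, it deactivates projectile movement and spawns a Niagara hit system at its transform, without destroying itself.
; The Niagara finish event only prints a debug string.
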(event OnComponentBeginOverlap(Sphere)
  (params (OverlappedComponent :type Primitive%20Component%20Object%20Reference) (OtherActor :type Actor%20Object%20Reference) (OtherComp :type Primitive%20Component%20Object%20Reference) (OtherBodyIndex :type Integer) (bFromSweep :type Boolean) (SweepResult :type Hit%20Result%20Structure%20%28by%20ref%29))
  (bind _returnvalue (Transformation|GetActorTransform))
  (if (not (Utilities|DoesObjectImplementInterface OtherActor "/Game/Core/Weapons/LeviathanAxe/BPI_ProjectilHit.BPI_ProjectilHit_C"))
    (Math|Integer|IncrementInt (Variables|Default|GetCount)
      (:%20%20
        (if (>= (Variables|Default|GetCount) 3)
          (Components|Activation|Deactivate (Variables|Default|GetProjectileMovement))
          (Niagara|SpawnSystematLocation "/Game/Core/Weapons/LeviathanAxe/VFX/sA_IceSkillPack2/Fx/NS_Projectile_Hit_1.NS_Projectile_Hit_1" (.location _returnvalue) (.rotation _returnvalue) (.scale _returnvalue)))))))

(event OnSystemFinished(Niagara)
  (params (PSystem :type Niagara%20Component%20Object%20Reference))
  (Development|PrintString "finiss"))

(event EventBeginPlay)

(event Collision|EventActorBeginOverlap
  (params (OtherActor :type Actor%20Object%20Reference)))

(event EventTick
  (params (DeltaSeconds :type Float%20%28single-precision%29)))

(fn ConstructionScript)