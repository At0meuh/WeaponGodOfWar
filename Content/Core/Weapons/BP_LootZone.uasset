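; BP_LootZone is a weapon pickup zone that hands its WeaponToLoot to an actor entering its box.
; On overlap, actors implementing BPI_Interraction receive EquipWeaponMessage with that weapon, then the zone destroys itself.
; EditorSetLootLocation moves the referenced weapon actor to the zone's location.
; The Destroyed event only prints a debug "Hello".
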(event OnComponentBeginOverlap(Box)
  (params (OverlappedComponent :type Primitive%20Component%20Object%20Reference) (OtherActor :type Actor%20Object%20Reference) (OtherComp :type Primitive%20Component%20Object%20Reference) (OtherBodyIndex :type Integer) (bFromSweep :type Boolean) (SweepResult :type Hit%20Result%20Structure%20%28by%20ref%29))
  (if (Utilities|DoesObjectImplementInterface OtherActor "/Game/Core/Player/BPI_Interraction.BPI_Interraction_C")
    (Class|BPIInterraction|EquipWeapon(Message) OtherActor (Variables|Default|GetWeaponToLoot))
    (Actor|DestroyActor)))

(event Custom|EditorSetLootLocation
  (Transformation|SetActorLocation (Variables|Default|GetWeaponToLoot) (Transformation|GetActorLocation) false false))

(event EventBeginPlay)

(event Collision|EventActorBeginOverlap
  (params (OtherActor :type Actor%20Object%20Reference)))

(event EventTick
  (params (DeltaSeconds :type Float%20%28single-precision%29)))

(event EventDestroyed
  (Development|PrintString "Hello"))

(fn ConstructionScript)